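; Player character Blueprint for Aura, handling motion-warp facing, shock-loop state and fading of overlapped actors.
; UpdateFacingTarget feeds the FacingTarget warp location, and SetinShockLoop stores the loop flag.
; FadeBoxTop overlaps send fade-out and fade-in messages to actors implementing BI_FadeInterface.
; The IA_CamToggle camera switch is unfinished: it sets TogglingCam, but the camera swap and delayed reset are disconnected.
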(event OnComponentBeginOverlap(FadeBoxTop)
  (params (OverlappedComponent :type Primitive%20Component%20Object%20Reference) (OtherActor :type Actor%20Object%20Reference) (OtherComp :type Primitive%20Component%20Object%20Reference) (OtherBodyIndex :type Integer) (bFromSweep :type Boolean) (SweepResult :type Hit%20Result%20Structure%20%28by%20ref%29))
  (if (Utilities|DoesObjectImplementInterface OtherActor "/Game/BPs/Actor/FadeActor/BI_FadeInterface.BI_FadeInterface_C")
    (Class|BIFadeInterface|FadeOut(Message) OtherActor)))

(event OnComponentEndOverlap(FadeBoxTop)
  (params (OverlappedComponent :type Primitive%20Component%20Object%20Reference) (OtherActor :type Actor%20Object%20Reference) (OtherComp :type Primitive%20Component%20Object%20Reference) (OtherBodyIndex :type Integer))
  (if (Utilities|DoesObjectImplementInterface OtherActor "/Game/BPs/Actor/FadeActor/BI_FadeInterface.BI_FadeInterface_C")
    (Class|BIFadeInterface|Fadein(Message) OtherActor)))

(event Custom|SpawnCamSwitch
  ;[0.005 0.026 0.766] Camera Toggle
  (if (not (Variables|Default|GetTogglingCam))
    (Variables|Default|SetTogglingCam true)
    (if (Variables|Default|GetTopCamActive)
      _)))

(event Input|EnhancedActionEvents|EnhancedInputActionIA_CamToggle
  (params (ActionValue :type Boolean) (ElapsedSeconds :type Float%20%28double-precision%29) (TriggeredSeconds :type Float%20%28double-precision%29) (InputAction :type Input%20Action%20Object%20Reference :default "/Game/BPs/Input/InputActions/IA_CamToggle.IA_CamToggle"))
  ;[0.005 0.026 0.766] Camera Toggle
  (:Triggered
    (if (not (Variables|Default|GetTogglingCam))
      (Variables|Default|SetTogglingCam true)
      (if (Variables|Default|GetTopCamActive)
        _))))

(event EventBeginPlay)

(event EventLevelUp)

(event EventSetinShockLoop
  (params (bInLoop :type Boolean))
  (Variables|Default|SetInShockLoop bInLoop))

(event EventUpdateFacingTarget
  (params (Target :type Vector%20%28by%20ref%29 :default "0, 0, 0"))
  (Class|MotionWarpingComponent|AddorUpdateWarpTargetfromLocation (Variables|Default|GetMotionWarping) "FacingTarget" Target))

(fn ConstructionScript)