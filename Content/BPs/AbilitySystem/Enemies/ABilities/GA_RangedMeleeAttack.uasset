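; Enemy gameplay ability that turns toward the combat target and performs a random tagged attack montage.
; A ranged tag skips the montage and applies a root-motion jump, ending on finish or landing.
; Other tags play the montage, await its gameplay event, then damage non-friendly live players near the combat socket.
; Any hit fires a MeleeImpact gameplay cue; the ability then ends.
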(event Custom|SetCallerByMagnitude
  ;[0.01096 0.01161 0.0137] ??? not needed ???
  (Ability|GameplayEffect|AssignTagSetbyCallerMagnitude (Ability|MakeOutgoingGameplayEffectSpec (Variables|Default|GetDamageEffectClass)) "(TagName=\"Damage.Physical\")" 0.0))

(event Ability|EventActivateAbility
  ;[0.02808 0.599 0.1382] Gameplay ABility Melee Attack
  (Variables|Default|SetHasHitTarget false)
  (bind _output_get (Variables|Default|SetAvatarActorInfo (Ability|GetAvatarActorfromActorInfo)))
  (bind _returnvalue (Class|EnemyInterface|GetCombatTarget(Message) _output_get))
  (bind _ascombat_interface (Utilities|Casting|CastToCombatInterface (Variables|Default|GetAvatarActorInfo)))
  (Class|CombatInterface|UpdateFacingTarget _ascombat_interface (Transformation|GetActorLocation _returnvalue))
  (bind _returnvalue_2 (Class|CombatInterface|GetAttackMontages(Message) (Variables|Default|GetAvatarActorInfo)))
  (bind _output_get_2 (Variables|Default|SetTaggedMontage (Class|AuraDamageGameplayAbility|GetRandomTaggedMontagefromArray _returnvalue_2)))
  (if (== (.MontageTag (Utilities|Struct|BreakTaggedMontage _output_get_2)) "(TagName=\"Montage.Attack.Ranged\")")
    (Development|PrintString (GameplayTags|GetDebugStringfromGameplayTag (.MontageTag (Utilities|Struct|BreakTaggedMontage _output_get_2))))
    (|ApplyRootMotionJumpForce "None" "0, 0, 0" 6e+02 1.5e+02 0.0 0.0 false "MaintainLastRootMotionVelocity" "0, 0, 0" 0.0
      (:OnFinish
        _)
      (:OnLanded
        _))
    (Ability|EndAbility)
    (else
      (|PlayMontageandWaitProxy "None" (.Montage (Utilities|Struct|BreakTaggedMontage _output_get_2)) 0.8 "Default" false 1.0 0.0
        (:then
          (Ability|Tasks|WaitGameplayEvent (.MontageTag (Utilities|Struct|BreakTaggedMontage _output_get_2)) 0
            (:EventReceived
              (bind _returnvalue_3 (Class|CombatInterface|GetCombatSocketLocation(Message) (Variables|Default|GetAvatarActorInfo) (.SocketTag (Utilities|Struct|BreakTaggedMontage _output_get_2))))
              (bind _output_get_3 (Variables|Default|SetCombatSocketLocation _returnvalue_3))
              (bind _outoverlappingactors (Class|AuraAbilitySystemLibrary|GetLivePlayersWithinRadius (Variables|Default|GetAvatarActorInfo) (Utilities|Array|MakeArray (Variables|Default|GetAvatarActorInfo)) 45.0 _output_get_3))
              (for _array_element _outoverlappingactors
                (if (Class|AuraAbilitySystemLibrary|IsNotFriend (Variables|Default|GetAvatarActorInfo) _array_element)
                  (Class|AuraDamageGameplayAbility|CauseDamage _array_element)
                  (Variables|Default|SetHasHitTarget true)))
              (if (Variables|Default|GetHasHitTarget)
                (bind _returnvalue_4 (Class|EnemyInterface|GetCombatTarget(Message) (Variables|Default|GetAvatarActorInfo)))
                (Variables|Default|SetCombatTarget _returnvalue_4)
                (Class|GameplayAbility|ExecuteGameplayCuewithParams "(TagName=\"GameplayCue.MeleeImpact\")" (Ability|GameplayCue|MakeGameplayCueParameters :AggregatedSourceTags (GameplayTags|MakeGameplayTagContainerfromTag (.MontageTag (Utilities|Struct|BreakTaggedMontage (Variables|Default|GetTaggedMontage)))) :Location (Variables|Default|GetCombatSocketLocation) :EffectCauser (Variables|Default|GetAvatarActorInfo) :SourceObject (Variables|Default|GetCombatTarget))))
              (Ability|EndAbility))))
        (:OnCompleted
          (Ability|EndAbility :!label _label))
        (:OnInterrupted
          (goto _label))
        (:OnCancelled
          (goto _label))))))