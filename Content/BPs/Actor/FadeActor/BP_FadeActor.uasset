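; BP_FadeActor is an actor that fades its mesh out and back in through material instances, triggering both on BeginPlay around a short delay.
; Construction stores original materials and creates dynamic instances from FadeMaterialInstances, which FadeOut applies by slot index.
; A timeline drives their "Fade" scalar, and FadeIn reverses it.
; On finish, a value of one restores original materials, and either endpoint sets Visibility collision to Block.
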(event Custom|FadeOut
  (CallFunction|SetMatstoDynamicInsts)
  (bind _fade (Timeline|Fade%20Out Play)
    (:Update
      (for _array_element (Variables|Default|GetMaterialInstanceDynamic)
        (Rendering|Material|SetScalarParameterValue _array_element "Fade" _fade :!class /Script/Engine.MaterialInstanceDynamic)))
    (:Finished
      (CallFunction|FadeFInished _fade))))

(event Custom|FadeIn
  (bind _fade (Timeline|Fade%20Out Reverse)
    (:Update
      (for _array_element (Variables|Default|GetMaterialInstanceDynamic)
        (Rendering|Material|SetScalarParameterValue _array_element "Fade" _fade :!class /Script/Engine.MaterialInstanceDynamic)))
    (:Finished
      (CallFunction|FadeFInished _fade))))

(event EventBeginPlay
  (CallFunction|FadeOut)
  (Utilities|FlowControl|Delay 1.1)
  (CallFunction|Fadein))

(event Collision|EventActorBeginOverlap
  (params (OtherActor :type Actor%20Object%20Reference)))

(event EventTick
  (params (DeltaSeconds :type Float%20%28single-precision%29)))

(fn ConstructionScript
  (Utilities|Array|Clear (Variables|Default|GetMaterialInstanceDynamic))
  (Variables|Default|SetOriginalMaterials (Rendering|Material|GetMaterials (Variables|Default|GetMesh)))
  (for _array_element (Variables|Default|GetFadeMaterialInstances)
    (bind _returnvalue (Rendering|Material|CreateDynamicMaterialInstance _array_element "None" "None" :!class /Script/Engine.KismetMaterialLibrary))
    (Utilities|Array|AddUnique (Variables|Default|GetMaterialInstanceDynamic) _returnvalue)))

(fn SetMatstoDynamicInsts
  (for (_array_element _array_index) (Variables|Default|GetMaterialInstanceDynamic)
    (Rendering|Material|SetMaterial (Variables|Default|GetMesh) _array_index _array_element)
    (return)))

(fn ResetMaterials
  (for (_array_element _array_index) (Variables|Default|GetOriginalMaterials)
    (Rendering|Material|SetMaterial (Variables|Default|GetMesh) _array_index _array_element)))

(fn FadeFInished
  (params (InputPin :type Float%20%28single-precision%29))
  (if (>= InputPin 1.0)
    (CallFunction|ResetMaterials)
    (Collision|SetCollisionResponsetoChannel (Variables|Default|GetMesh) "ECC_Visibility" "ECR_Block")
    (elif (<= InputPin 0.0)
      (Collision|SetCollisionResponsetoChannel (Variables|Default|GetMesh) "ECC_Visibility" "ECR_Block"))))