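; Base pawn Blueprint for gun factions, whose event graph is effectively inert.
; Input mapping context setup is noted as already handled in C++, leaving its Enhanced Input event here unused.
; Deprecated axis-based WASD_2 and mouse-look graphs remain unexecuted; they apply yaw-only planar movement and controller pitch/yaw.
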(event Custom|AssignInputMappingContext
  ;[0.05729 0.05729 0.573] Assign Input Mapping Context (Enhanced Input config) already set in CPP
  (bind _asplayer_controller (Utilities|Casting|CastToPlayerController (Pawn|GetController)))
  (Utilities|IsValid (PlayerController|LocalPlayerSubsystems|GetEnhancedInputLocalPlayerSubsystem _asplayer_controller)
    (:Is%20Valid
      (Input|AddMappingContext (PlayerController|LocalPlayerSubsystems|GetEnhancedInputLocalPlayerSubsystem _asplayer_controller) "/Game/BPs/ToTW/IMC_TotwContext.IMC_TotwContext" 0 "(bIgnoreAllPressedKeysUntilRelease=True,bForceImmediately=False)"))))

(event EventBeginPlay
  ;[0.02808 0.599 0.1382] BEGIN PLAY
)

(event Collision|EventActorBeginOverlap
  (params (OtherActor :type Actor%20Object%20Reference)))

(event EventTick
  (params (DeltaSeconds :type Float%20%28single-precision%29)))

(fn ConstructionScript)