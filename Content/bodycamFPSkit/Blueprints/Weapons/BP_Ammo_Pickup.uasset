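; Ammo pickup actor that adds reserve ammo to the first-person character's equipped primary or secondary weapon.
; Sphere overlap passes itself to the overlapping actor via InteractionMessage and, if the equipped slot holds a non-base weapon, enables taking and shows a "Press F" hint; leaving clears both.
; PickUp adds AmmoPickup to that slot's MaxAmmo, refreshes the weapon's ammo data and destroys the actor.
; The construction script applies the configurable mesh.
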(event OnComponentBeginOverlap(Sphere)
  (params (OverlappedComponent :type Primitive%20Component%20Object%20Reference) (OtherActor :type Actor%20Object%20Reference) (OtherComp :type Primitive%20Component%20Object%20Reference) (OtherBodyIndex :type Integer) (bFromSweep :type Boolean) (SweepResult :type Hit%20Result%20Structure%20%28by%20ref%29))
  (bind _as_first_person_character (Variables|Default|GetAs%20First%20Person%20Character))
  (bind _as_first_person_character_2 (Variables|Default|GetAs%20First%20Person%20Character))
  (bind _equippedweapon (Variables|/Game/bodycamFPSkit/Blueprints/BP_FirstPersonCharacter.BP_FirstPersonCharacter_C|GetEquippedWeapon _as_first_person_character_2))
  (bind _weaponslot_1 (Variables|/Game/bodycamFPSkit/Blueprints/BP_FirstPersonCharacter.BP_FirstPersonCharacter_C|GetWeaponSlot_1 _as_first_person_character))
  (bind _weaponslot_2 (Variables|/Game/bodycamFPSkit/Blueprints/BP_FirstPersonCharacter.BP_FirstPersonCharacter_C|GetWeaponSlot_2 _as_first_person_character))
  ;[0 0 0] Check Is The Player Can Take Weapon and Selects What To Do With Weapon
  (Variables|Default|SetCanPickUp true)
  (Class|INTInteraction|Interaction(Message) OtherActor self)
  (Utilities|FlowControl|Sequence
    (:then_0
      (if (Utilities|Enum|Equal(Enum) _equippedweapon "NewEnumerator0")
        (if (not (== (.WeaponData (Utilities|Struct|BreakST_WeaponStats _weaponslot_1)) "/Game/bodycamFPSkit/Blueprints/Weapons/BP_Weapon_Base.BP_Weapon_Base_C"))
          (Development|PrintString "take ammo" :!label _label)
          (Variables|Default|SetTakeAmmo true)
          (Variables|/Game/bodycamFPSkit/Blueprints/BP_FirstPersonCharacter.BP_FirstPersonCharacter_C|SetWeaponChangeHint (Variables|Default|GetAs%20First%20Person%20Character) (Utilities|String|Append "Press \"F\" to Take Ammo for " (.WeaponName (Utilities|Struct|BreakST_WeaponStats (Utilities|Select :Index (Variables|/Game/bodycamFPSkit/Blueprints/BP_FirstPersonCharacter.BP_FirstPersonCharacter_C|GetEquippedWeapon (Variables|Default|GetAs%20First%20Person%20Character)) :NewEnumerator7 "" :NewEnumerator0 _weaponslot_1 :NewEnumerator1 _weaponslot_2))))))))
    (:then_1
      (if (Utilities|Enum|Equal(Enum) _equippedweapon "NewEnumerator1")
        (if (not (== (.WeaponData (Utilities|Struct|BreakST_WeaponStats _weaponslot_2)) "/Game/bodycamFPSkit/Blueprints/Weapons/BP_Weapon_Base.BP_Weapon_Base_C"))
          (goto _label))))))

(event OnComponentEndOverlap(Sphere)
  (params (OverlappedComponent :type Primitive%20Component%20Object%20Reference) (OtherActor :type Actor%20Object%20Reference) (OtherComp :type Primitive%20Component%20Object%20Reference) (OtherBodyIndex :type Integer))
  ;[0 0 0] Check Is The Player Can Take Weapon and Selects What To Do With Weapon
  (Variables|Default|SetCanPickUp false)
  (Variables|Default|SetTakeAmmo false)
  (Variables|/Game/bodycamFPSkit/Blueprints/BP_FirstPersonCharacter.BP_FirstPersonCharacter_C|SetWeaponChangeHint (Variables|Default|GetAs%20First%20Person%20Character) ""))

(event Custom|WeaponToAmmo
  (bind _as_first_person_character (Variables|Default|GetAs%20First%20Person%20Character))
  (bind _as_first_person_character_2 (Variables|Default|GetAs%20First%20Person%20Character))
  (bind _ammopickup (Variables|WeaponVars|GetAmmoPickup))
  (bind _as_first_person_character_3 (Variables|Default|GetAs%20First%20Person%20Character))
  (bind _equippedweapon (Variables|/Game/bodycamFPSkit/Blueprints/BP_FirstPersonCharacter.BP_FirstPersonCharacter_C|GetEquippedWeapon _as_first_person_character))
  ;[0 0 0] Add Ammo to Gun
  (if (Utilities|Enum|Equal(Enum) _equippedweapon "NewEnumerator0")
    (Variables|/Game/bodycamFPSkit/Blueprints/BP_FirstPersonCharacter.BP_FirstPersonCharacter_C|SetWeaponSlot_1 _as_first_person_character_3 (Utilities|Struct|MakeST_WeaponStats (.AmmoCount (Utilities|Struct|BreakST_WeaponStats (Variables|/Game/bodycamFPSkit/Blueprints/BP_FirstPersonCharacter.BP_FirstPersonCharacter_C|GetWeaponSlot_1 _as_first_person_character_2))) (+ (.MaxAmmo (Utilities|Struct|BreakST_WeaponStats (Variables|/Game/bodycamFPSkit/Blueprints/BP_FirstPersonCharacter.BP_FirstPersonCharacter_C|GetWeaponSlot_1 _as_first_person_character_2))) _ammopickup) (.WeaponData (Utilities|Struct|BreakST_WeaponStats (Variables|/Game/bodycamFPSkit/Blueprints/BP_FirstPersonCharacter.BP_FirstPersonCharacter_C|GetWeaponSlot_1 _as_first_person_character_2))) "NewEnumerator0" (.WeaponName (Utilities|Struct|BreakST_WeaponStats (Variables|/Game/bodycamFPSkit/Blueprints/BP_FirstPersonCharacter.BP_FirstPersonCharacter_C|GetWeaponSlot_1 _as_first_person_character_2)))))
    (Default|SetWeaponAmmoData (Default|GetWeapon (Variables|Default|GetAs%20First%20Person%20Character)) true :!label _label)
    (elif (Utilities|Enum|Equal(Enum) _equippedweapon "NewEnumerator1")
      (Variables|/Game/bodycamFPSkit/Blueprints/BP_FirstPersonCharacter.BP_FirstPersonCharacter_C|SetWeaponSlot_2 _as_first_person_character_3 (Utilities|Struct|MakeST_WeaponStats (.AmmoCount (Utilities|Struct|BreakST_WeaponStats (Variables|/Game/bodycamFPSkit/Blueprints/BP_FirstPersonCharacter.BP_FirstPersonCharacter_C|GetWeaponSlot_2 _as_first_person_character_2))) (+ (.MaxAmmo (Utilities|Struct|BreakST_WeaponStats (Variables|/Game/bodycamFPSkit/Blueprints/BP_FirstPersonCharacter.BP_FirstPersonCharacter_C|GetWeaponSlot_2 _as_first_person_character_2))) _ammopickup) (.WeaponData (Utilities|Struct|BreakST_WeaponStats (Variables|/Game/bodycamFPSkit/Blueprints/BP_FirstPersonCharacter.BP_FirstPersonCharacter_C|GetWeaponSlot_2 _as_first_person_character_2))) "NewEnumerator1" (.WeaponName (Utilities|Struct|BreakST_WeaponStats (Variables|/Game/bodycamFPSkit/Blueprints/BP_FirstPersonCharacter.BP_FirstPersonCharacter_C|GetWeaponSlot_2 _as_first_person_character_2)))))
      (goto _label))))

(event EventPickUp
  ;[0 0 0] Pickup Ammo
  (if (Variables|Default|GetCanPickUp)
    (if (Variables|Default|GetTakeAmmo)
      (CallFunction|WeapontoAmmo)
      (Actor|DestroyActor))))

(fn ConstructionScript
  (|CallParentFunction)
  (Components|StaticMesh|SetStaticMesh (Variables|Default|GetAmmo) (Variables|WeaponVars|GetAmmoMesh)))