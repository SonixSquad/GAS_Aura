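; Base weapon for the bodycam FPS character, with empty fire, reload, inspect and melee events and shared hitscan, aiming and ammo-slot sync logic.
; Timelines drive procedural equip/stow and low/high poses by writing offsets to the parent character.
; Hitscan traces from muzzle or camera with spread and shotgun pellets, spawning impacts, decals and casings but applying no damage.
; Aim hand transforms are computed from tagged optic and front/rear sight sockets.
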(event Custom|FinishReload
  ;[0 0 0] Events
)

(event Custom|Equip
  (bind _playerref (Variables|Character|GetPlayerRef))
  (bind _playerref_2 (Variables|Character|GetPlayerRef))
  ;[0 0 0] Events
  ;[0 0 0] Set Recoil Values
  (Variables|/Game/bodycamFPSkit/Blueprints/BP_FirstPersonCharacter.BP_FirstPersonCharacter_C|SetRecoilValues (Variables|Character|GetPlayerRef) (Variables|FireLogic|GetRecoilVars))
  ;[0 0 0] Weapon Hand Transform
  (Variables|/Game/bodycamFPSkit/Blueprints/BP_FirstPersonCharacter.BP_FirstPersonCharacter_C|SetWeaponLocation _playerref (Variables|ProceduralAnims|GetWeaponLocation))
  (Variables|/Game/bodycamFPSkit/Blueprints/BP_FirstPersonCharacter.BP_FirstPersonCharacter_C|SetWeaponRotation _playerref (Variables|ProceduralAnims|GetWeaponRotation))
  ;[0 0 0] Check The Character Have Weapon
  (if (Variables|Default|GetIsWeapon)
    (Variables|ProceduralAnims|SetEquipped true)
    ;[0 0 0] Update Player ADS Offset
    (Variables|/Game/bodycamFPSkit/Blueprints/BP_FirstPersonCharacter.BP_FirstPersonCharacter_C|SetADS_Offset (Variables|Character|GetPlayerRef) (Variables|ADS|GetADS_Offset))
    ;[0 0 0] Procedural Equip Via Timeline
    (Audio|PlaySound2D (Variables|Audio|GetEquipSound) 1.0 1.0 0.0 0 0)
    (bind (_direction _updownalpha _rollalpha) (Timeline|TL_Equip/Stow PlayFromStart)
      (:Update
        (if (Variables|Default|GetIsWeapon)
          (Variables|/Game/bodycamFPSkit/Blueprints/BP_FirstPersonCharacter.BP_FirstPersonCharacter_C|SetEquipLoc _playerref_2 (Math|Vector|MakeVector 0.0 0.0 _updownalpha))
          (Variables|/Game/bodycamFPSkit/Blueprints/BP_FirstPersonCharacter.BP_FirstPersonCharacter_C|SetEquipRot _playerref_2 (Math|Rotator|MakeRotator _rollalpha _rollalpha (* _rollalpha -5.0)))
          (else
            (Variables|/Game/bodycamFPSkit/Blueprints/BP_FirstPersonCharacter.BP_FirstPersonCharacter_C|SetEquipLoc _playerref_2 "0, 0, 0")
            (Variables|/Game/bodycamFPSkit/Blueprints/BP_FirstPersonCharacter.BP_FirstPersonCharacter_C|SetEquipRot _playerref_2 "0, 0, 0")))
        (Default|SetCharacterSpeed (Variables|Character|GetPlayerRef))))))

(event Custom|Inspect
  ;[0 0 0] Events
)

(event Custom|Reload
  ;[0 0 0] Events
)

(event Custom|Stow
  (bind _playerref (Variables|Character|GetPlayerRef))
  ;[0 0 0] Events
  ;[0 0 0] Check The Character Have Weapon
  (if (Variables|Default|GetIsWeapon)
    (Variables|ProceduralAnims|SetEquipped false)
    ;[0 0 0] Procedural Equip Via Timeline
    (Audio|PlaySound2D (Variables|Audio|GetUnequipSound) 1.0 1.0 0.0 0 0)
    (bind (_direction _updownalpha _rollalpha) (Timeline|TL_Equip/Stow ReverseFromEnd)
      (:Update
        (if (Variables|Default|GetIsWeapon)
          (Variables|/Game/bodycamFPSkit/Blueprints/BP_FirstPersonCharacter.BP_FirstPersonCharacter_C|SetEquipLoc _playerref (Math|Vector|MakeVector 0.0 0.0 _updownalpha))
          (Variables|/Game/bodycamFPSkit/Blueprints/BP_FirstPersonCharacter.BP_FirstPersonCharacter_C|SetEquipRot _playerref (Math|Rotator|MakeRotator _rollalpha _rollalpha (* _rollalpha -5.0)))
          (else
            (Variables|/Game/bodycamFPSkit/Blueprints/BP_FirstPersonCharacter.BP_FirstPersonCharacter_C|SetEquipLoc _playerref "0, 0, 0")
            (Variables|/Game/bodycamFPSkit/Blueprints/BP_FirstPersonCharacter.BP_FirstPersonCharacter_C|SetEquipRot _playerref "0, 0, 0")))
        (Default|SetCharacterSpeed (Variables|Character|GetPlayerRef))))))

(event Custom|ChangeSight
  (bind _opticsight (Variables|Default|GetOpticSight))
  (bind _handtransforms (Variables|ADS|GetHandTransforms))
  ;[0 0 0] Check the Sights Character Have and Change It
  (if (> (Utilities|Array|Length _handtransforms) 0)
    (if (> (Utilities|Array|LastIndex _handtransforms) (Variables|ADS|GetCurrentSight))
      (Math|Integer|IncrementInt (Variables|ADS|GetCurrentSight)
        (:%20%20
          (Rendering|SetVisibility _opticsight false false)))
      (else
        (Variables|ADS|SetCurrentSight 0)
        (Rendering|SetVisibility _opticsight true false)))))

(event Custom|StopFire
  ;[0 0 0] Events
)

(event Custom|High
  (bind _playerref (Variables|Character|GetPlayerRef))
  (bind _runposerot (Variables|ProceduralAnims|GetRunPoseRot))
  ;[0 0 0] Events
  ;[0 0 0] Check The Character Have Weapon
  (if (Variables|Default|GetIsWeapon)
    (Variables|ProceduralAnims|SetIsLow false)
    ;[0 0 0] Procedural Low High and Running Via Timeline with Variables
    (Audio|PlaySound2D (Variables|Audio|GetHighSound) 1.0 1.0 0.0 0 0)
    (bind _updownalpha (Timeline|TL_Low/High ReverseFromEnd)
      (:Update
        (Variables|/Game/bodycamFPSkit/Blueprints/BP_FirstPersonCharacter.BP_FirstPersonCharacter_C|SetLowHighLoc _playerref (Math|Vector|MakeVector (* _updownalpha (Variables|ProceduralAnims|GetRunPoseRight)) (Variables|ProceduralAnims|GetRunPoseFront) (Variables|ProceduralAnims|GetRunPoseHeight)))
        (Variables|/Game/bodycamFPSkit/Blueprints/BP_FirstPersonCharacter.BP_FirstPersonCharacter_C|SetLowHighRot _playerref (Math|Rotator|MakeRotator (.roll _runposerot) (.pitch _runposerot) (.yaw _runposerot)))))))

(event Custom|Low
  (bind _playerref (Variables|Character|GetPlayerRef))
  (bind _runposerot (Variables|ProceduralAnims|GetRunPoseRot))
  ;[0 0 0] Events
  ;[0 0 0] Check The Character Have Weapon
  (if (Variables|Default|GetIsWeapon)
    (Variables|ProceduralAnims|SetIsLow true)
    ;[0 0 0] Procedural Low High and Running Via Timeline with Variables
    (Audio|PlaySound2D (Variables|Audio|GetLowSound) 1.0 1.0 0.0 0 0)
    (bind _updownalpha (Timeline|TL_Low/High PlayFromStart)
      (:Update
        (Variables|/Game/bodycamFPSkit/Blueprints/BP_FirstPersonCharacter.BP_FirstPersonCharacter_C|SetLowHighLoc _playerref (Math|Vector|MakeVector (* _updownalpha (Variables|ProceduralAnims|GetRunPoseRight)) (Variables|ProceduralAnims|GetRunPoseFront) (Variables|ProceduralAnims|GetRunPoseHeight)))
        (Variables|/Game/bodycamFPSkit/Blueprints/BP_FirstPersonCharacter.BP_FirstPersonCharacter_C|SetLowHighRot _playerref (Math|Rotator|MakeRotator (.roll _runposerot) (.pitch _runposerot) (.yaw _runposerot)))))))

(event Custom|Melee
  ;[0 0 0] Events
)

(event Custom|Fire
  ;[0 0 0] Events
)

(event EventBeginPlay
  (bind _returnvalue (Actor|GetParentActor))
  ;[0 0 0] Get Player Referance
  (Utilities|FlowControl|Sequence
    (:then_0
      (bind _asaura_player_state (Utilities|Casting|CastToAuraPlayerState _returnvalue))
      (Development|PrintString (PlayerState|GetPlayerName _asaura_player_state)))
    (:then_1
      (bind _asbp_first_person_character (Utilities|Casting|CastToBP_FirstPersonCharacter _returnvalue))
      (Variables|Character|SetPlayerRef _asbp_first_person_character)
      ;[0 0 0] Setup Equip and Stow Speed
      (Components|Timeline|SetPlayRate (Variables|Default|GetTL_Equip/Stow) (Variables|ProceduralAnims|GetEquip/StowSpeed))
      (CallFunction|Equip)
      (Default|SocketOffset (Variables|Character|GetPlayerRef) (Variables|WeaponStats|GetHand_R_SocketOffset)))))

(fn ConstructionScript
  (Components|SkinnedMesh|SetSkinnedAssetandUpdate (Variables|Default|GetWeapon_Mesh) (Variables|Weapon|GetMesh) true)
  (Rendering|SetVisibility (Variables|Default|GetSpareMag) false false)
  ;[0 0 0] Attach Optic Sight To Slide Bone On The Weapon
  (Transformation|AttachComponentToComponent (Variables|Default|GetOpticSight) (Variables|Default|GetWeapon_Mesh) "slide" "KeepRelative" "KeepRelative" "KeepRelative" false)
  (if (!= (Variables|Weapon|GetSpareMagMesh) 0)
    (Components|StaticMesh|SetStaticMesh (Variables|Default|GetSpareMag) (Variables|Weapon|GetSpareMagMesh))
    (Transformation|AttachComponentToComponent (Variables|Default|GetSpareMag) (Variables|Default|GetWeapon_Mesh) (Variables|Weapon|GetSpareMagSocket) "SnapToTarget" "SnapToTarget" "SnapToTarget" false)))

(fn FireHitScan
  (params (DrawDebug :type Boolean) (Range :type Float%20%28double-precision%29) (TraceStyle :type ENUM_LineTraceStyles%20Enum :default "NewEnumerator7") (IsMelee :type Boolean) (IsShotgun :type Boolean))
  (bind _playerref (Variables|Character|GetPlayerRef))
  (bind _spread (Variables|WeaponStats|GetSpread))
  (bind _spread_2 (Variables|WeaponStats|GetSpread))
  (bind _weapon_mesh (Variables|Default|GetWeapon_Mesh))
  (bind _weapon_mesh_2 (Variables|Default|GetWeapon_Mesh))
  (bind _returnvalue (Transformation|GetSocketLocation _weapon_mesh_2 "Muzzle"))
  (bind _returnvalue_2 (Transformation|GetSocketRotation _weapon_mesh_2 "Muzzle"))
  (bind _returnvalue_3 (Transformation|GetSocketTransform _weapon_mesh "BulletCasing" "RTS_World"))
  (bind _firstpersoncamera (Variables|/Game/bodycamFPSkit/Blueprints/BP_FirstPersonCharacter.BP_FirstPersonCharacter_C|GetFirstPersonCamera _playerref))
  (bind _returnvalue_4 (Transformation|GetWorldLocation _firstpersoncamera))
  (bind _returnvalue_5 (Math|Vector|GetForwardVector _firstpersoncamera))
  (bind _returnvalue_6 (Math|Vector|GetForwardVector _returnvalue_2))
  (bind _returnvalue_7 (Math|Random|RandomUnitVectorinConeinDegrees _returnvalue_6 _spread_2))
  (bind _returnvalue_8 (Math|Random|RandomUnitVectorinConeinDegrees _returnvalue_5 _spread))
  (bind _returnvalue_9 (* _returnvalue_7 Range))
  (bind _returnvalue_10 (* _returnvalue_8 Range))
  (bind _returnvalue_11 (+ _returnvalue_4 _returnvalue_10))
  (bind _returnvalue_12 (+ _returnvalue _returnvalue_9))
  (bind (_x _y _z) (Math|Vector|BreakVector _returnvalue_11))
  (bind (_x_2 _y_2 _z_2) (Math|Vector|BreakVector _returnvalue_12))
  ;[0 0 0] LineTrace from Camera
  (Variables|Default|SetDrawDebug DrawDebug)
  (if IsShotgun
    (for _index (range 1 7)
      (switch Utilities|FlowControl|Switch|SwitchonENUM_LineTraceStyles TraceStyle
        (:NewEnumerator7
          ;[0 0 0] Linetrace from Weapon Muzzle
          (bind _outhit (Collision|LineTraceByChannel _returnvalue (Math|Vector|SelectVector (Math|Vector|MakeVector _x_2 (+ _y_2 (Math|Random|RandomFloatinRange -3.5e+02 3.5e+02)) (+ _z_2 (Math|Random|RandomFloatinRange -3.5e+02 3.5e+02))) _returnvalue_12 IsShotgun) "TraceTypeQuery1" false (Utilities|Array|MakeArray (Variables|Character|GetPlayerRef)) (select (Variables|Default|GetDrawDebug) "ForDuration" "None"))))
        (:NewEnumerator0
          (bind _outhit_2 (Collision|LineTraceByChannel _returnvalue_4 (Math|Vector|SelectVector (Math|Vector|MakeVector _x (+ _y (Math|Random|RandomFloatinRange -3.5e+02 3.5e+02)) (+ _z (Math|Random|RandomFloatinRange -3.5e+02 3.5e+02))) _returnvalue_11 IsShotgun) "TraceTypeQuery1" false (Utilities|Array|MakeArray (Variables|Character|GetPlayerRef)) (select (Variables|Default|GetDrawDebug) "ForDuration" "None")))))
      (if (not IsMelee)
        (Utilities|FlowControl|Sequence
          (:then_0
            (Effects|SpawnEmitteratLocation "/Game/bodycamFPSkit/ParticleEffects/P_BulletImpact.P_BulletImpact" (.ImpactPoint (Collision|BreakHitResult (Utilities|Select :Index TraceStyle :NewEnumerator7 _outhit :NewEnumerator0 _outhit_2))) (Math|Conversions|RotationFromXVector (.ImpactNormal (Collision|BreakHitResult (Utilities|Select :Index TraceStyle :NewEnumerator7 _outhit :NewEnumerator0 _outhit_2)))) "1.000000,1.000000,1.000000" true "AutoRelease"))
          (:then_1
            (bind _returnvalue_13 (Class|GameplayStatics|SpawnDecalAttached "/Game/bodycamFPSkit/ParticleEffects/Materials/Mat_Impact_Decal.Mat_Impact_Decal" "1.000000,5.000000,5.000000" (.HitComponent (Collision|BreakHitResult (Utilities|Select :Index TraceStyle :NewEnumerator7 _outhit :NewEnumerator0 _outhit_2))) "None" (.ImpactPoint (Collision|BreakHitResult (Utilities|Select :Index TraceStyle :NewEnumerator7 _outhit :NewEnumerator0 _outhit_2))) (Math|Conversions|RotationFromXVector (.ImpactNormal (Collision|BreakHitResult (Utilities|Select :Index TraceStyle :NewEnumerator7 _outhit :NewEnumerator0 _outhit_2)))) "KeepWorldPosition" 15.0))
            (Utilities|IsValid _returnvalue_13
              (:Is%20Valid
                (Rendering|Components|Decal|SetFadeScreenSize _returnvalue_13 0.0))))
          (:then_2
            (Utilities|FlowControl|DoOnce false
              (:Completed
                (Effects|SpawnEmitteratLocation (Variables|Weapon|GetBulletCasing) (.location _returnvalue_3) (.rotation _returnvalue_3) "1.000000,1.000000,1.000000" true "AutoRelease")))))))
    (Utilities|FlowControl|DoOnce false) ; enters at Reset
    (else
      (switch Utilities|FlowControl|Switch|SwitchonENUM_LineTraceStyles TraceStyle
        (:NewEnumerator7
          (bind _outhit_3 (Collision|LineTraceByChannel _returnvalue (Math|Vector|SelectVector (Math|Vector|MakeVector _x_2 (+ _y_2 (Math|Random|RandomFloatinRange -3.5e+02 3.5e+02)) (+ _z_2 (Math|Random|RandomFloatinRange -3.5e+02 3.5e+02))) _returnvalue_12 IsShotgun) "TraceTypeQuery1" false (Utilities|Array|MakeArray (Variables|Character|GetPlayerRef)) (select (Variables|Default|GetDrawDebug) "ForDuration" "None"))))
        (:NewEnumerator0
          (bind _outhit_4 (Collision|LineTraceByChannel _returnvalue_4 (Math|Vector|SelectVector (Math|Vector|MakeVector _x (+ _y (Math|Random|RandomFloatinRange -3.5e+02 3.5e+02)) (+ _z (Math|Random|RandomFloatinRange -3.5e+02 3.5e+02))) _returnvalue_11 IsShotgun) "TraceTypeQuery1" false (Utilities|Array|MakeArray (Variables|Character|GetPlayerRef)) (select (Variables|Default|GetDrawDebug) "ForDuration" "None")))))
      (if (not IsMelee)
        (Utilities|FlowControl|Sequence
          (:then_0
            (Effects|SpawnEmitteratLocation "/Game/bodycamFPSkit/ParticleEffects/P_BulletImpact.P_BulletImpact" (.ImpactPoint (Collision|BreakHitResult (Utilities|Select :Index TraceStyle :NewEnumerator7 _outhit_3 :NewEnumerator0 _outhit_4))) (Math|Conversions|RotationFromXVector (.ImpactNormal (Collision|BreakHitResult (Utilities|Select :Index TraceStyle :NewEnumerator7 _outhit_3 :NewEnumerator0 _outhit_4)))) "1.000000,1.000000,1.000000" true "AutoRelease"))
          (:then_1
            (bind _returnvalue_14 (Class|GameplayStatics|SpawnDecalAttached "/Game/bodycamFPSkit/ParticleEffects/Materials/Mat_Impact_Decal.Mat_Impact_Decal" "1.000000,5.000000,5.000000" (.HitComponent (Collision|BreakHitResult (Utilities|Select :Index TraceStyle :NewEnumerator7 _outhit_3 :NewEnumerator0 _outhit_4))) "None" (.ImpactPoint (Collision|BreakHitResult (Utilities|Select :Index TraceStyle :NewEnumerator7 _outhit_3 :NewEnumerator0 _outhit_4))) (Math|Conversions|RotationFromXVector (.ImpactNormal (Collision|BreakHitResult (Utilities|Select :Index TraceStyle :NewEnumerator7 _outhit_3 :NewEnumerator0 _outhit_4)))) "KeepWorldPosition" 15.0))
            (Utilities|IsValid _returnvalue_14
              (:Is%20Valid
                (Rendering|Components|Decal|SetFadeScreenSize _returnvalue_14 0.0))))
          (:then_2
            (Utilities|FlowControl|DoOnce false
              (:Completed
                (Effects|SpawnEmitteratLocation (Variables|Weapon|GetBulletCasing) (.location _returnvalue_3) (.rotation _returnvalue_3) "1.000000,1.000000,1.000000" true "AutoRelease")))))))))

(fn CalculateAIM
  (|CalculateOpticTransform
    (:output
      (|CalculateSightTransform
        (:output
          (return))))))

(fn SetWeaponAmmoData
  (params (IsPickUp :type Boolean))
  (bind _playerref (Variables|Character|GetPlayerRef))
  (bind _playerref_2 (Variables|Character|GetPlayerRef))
  (bind _playerref_3 (Variables|Character|GetPlayerRef))
  (bind _playerref_4 (Variables|Character|GetPlayerRef))
  (bind _playerref_5 (Variables|Character|GetPlayerRef))
  (bind _playerref_6 (Variables|Character|GetPlayerRef))
  (bind _weapon (Default|GetWeapon _playerref_5))
  (bind _equippedweapon (Variables|/Game/bodycamFPSkit/Blueprints/BP_FirstPersonCharacter.BP_FirstPersonCharacter_C|GetEquippedWeapon _playerref_4))
  (bind _equippedweapon_2 (Variables|/Game/bodycamFPSkit/Blueprints/BP_FirstPersonCharacter.BP_FirstPersonCharacter_C|GetEquippedWeapon _playerref_3))
  (bind _returnvalue (Utilities|GetClass _weapon))
  (if IsPickUp
    ;[0 0 0] ADDS AMMO TO WEAPON BLUEPRINT FROM PICKUP
    (if (Utilities|Enum|Equal(Enum) _equippedweapon "NewEnumerator0")
      (Variables|WeaponStats|SetAmmoCount (.ammocount (Variables|/Game/bodycamFPSkit/Blueprints/BP_FirstPersonCharacter.BP_FirstPersonCharacter_C|GetWeaponSlot_1 _playerref_2)))
      (Variables|WeaponStats|SetMaxAmmo (.maxammo (Variables|/Game/bodycamFPSkit/Blueprints/BP_FirstPersonCharacter.BP_FirstPersonCharacter_C|GetWeaponSlot_1 _playerref_2)))
      (elif (Utilities|Enum|Equal(Enum) _equippedweapon "NewEnumerator1")
        (Variables|WeaponStats|SetAmmoCount (.ammocount (Variables|/Game/bodycamFPSkit/Blueprints/BP_FirstPersonCharacter.BP_FirstPersonCharacter_C|GetWeaponSlot_2 _playerref_2)))
        (Variables|WeaponStats|SetMaxAmmo (.maxammo (Variables|/Game/bodycamFPSkit/Blueprints/BP_FirstPersonCharacter.BP_FirstPersonCharacter_C|GetWeaponSlot_2 _playerref_2)))))
    (else
      ;[0 0 0] SETUP AMMO ON THE CHARACTER BLUEPRINT FROM WEAPON BLUEPRINT (Checks the ammo you have every time you fired your weapon or reloading)
      (if (Utilities|Enum|Equal(Enum) _equippedweapon_2 "NewEnumerator0")
        (Variables|/Game/bodycamFPSkit/Blueprints/BP_FirstPersonCharacter.BP_FirstPersonCharacter_C|SetWeaponSlot_1 _playerref_6 (Utilities|Struct|MakeST_WeaponStats (Variables|WeaponStats|GetAmmoCount) (Variables|WeaponStats|GetMaxAmmo) _returnvalue "NewEnumerator0" (.weaponname (Variables|/Game/bodycamFPSkit/Blueprints/BP_FirstPersonCharacter.BP_FirstPersonCharacter_C|GetWeaponSlot_1 _playerref))))
        (elif (Utilities|Enum|Equal(Enum) _equippedweapon_2 "NewEnumerator1")
          (Variables|/Game/bodycamFPSkit/Blueprints/BP_FirstPersonCharacter.BP_FirstPersonCharacter_C|SetWeaponSlot_2 _playerref_6 (Utilities|Struct|MakeST_WeaponStats (Variables|WeaponStats|GetAmmoCount) (Variables|WeaponStats|GetMaxAmmo) _returnvalue "NewEnumerator1" (.weaponname (Variables|/Game/bodycamFPSkit/Blueprints/BP_FirstPersonCharacter.BP_FirstPersonCharacter_C|GetWeaponSlot_2 _playerref)))))))))