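; Free-aim component for the bodycam FPS kit that rotates an effector component from mouse input within a deadzone.
; While active, it scales input, caps horizontal to ±1, and accumulates per-axis rotations with angle clamps.
; The effector lerps toward that target, and the result is stored as the final aim rotation.
; Optional tilt adds a second lerp, but its target reads only TiltAroundX's zero roll and yaw, easing toward neutral.
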(fn FreeAimComponent
  (params (EffectorComponent :type Scene%20Component%20Object%20Reference) (HorizontalMouse :type Float%20%28double-precision%29) (VerticalMouse :type Float%20%28double-precision%29) (Speed :type Float%20%28double-precision%29) (IsActive :type Boolean))
  (if IsActive
    (Variables|InputValues|SetEffector%20Component EffectorComponent)
    (Variables|InputValues|SetHorizontal%20Mouse (* HorizontalMouse Speed))
    (Variables|InputValues|SetVertical%20Mouse (* VerticalMouse Speed))
    (Utilities|FlowControl|Sequence
      (:then_0
        (Utilities|FlowControl|Sequence
          (:then_0
            (if (> (Variables|InputValues|GetHorizontal%20Mouse) 1.0)
              (Variables|InputValues|SetHorizontal%20Mouse 1.0)))
          (:then_1
            (if (< (Variables|InputValues|GetHorizontal%20Mouse) -1.0)
              (Variables|InputValues|SetHorizontal%20Mouse -1.0)))))
      (:then_1
        (if (Variables|FreeAim|GetEnableDeadzoneX)
          (Variables|FreeAim|SetRotX (Math|Rotator|MakeRotator (+ (* (Variables|InputValues|GetHorizontal%20Mouse) (Variables|FreeAim|GetStartSensitivity)) (.Roll (Math|Rotator|BreakRotator (Variables|FreeAim|GetRotX)))) (+ (* (Variables|InputValues|GetHorizontal%20Mouse) (Variables|FreeAim|GetStartSensitivity)) (.Pitch (Math|Rotator|BreakRotator (Variables|FreeAim|GetRotX)))) (+ (* (Variables|InputValues|GetHorizontal%20Mouse) (Variables|FreeAim|GetStartSensitivity)) (.Yaw (Math|Rotator|BreakRotator (Variables|FreeAim|GetRotX))))))
          (Variables|FreeAim|SetRotX (Math|Rotator|MakeRotator (Math|Float|ClampAngle (.Roll (Math|Rotator|BreakRotator (Variables|FreeAim|GetRotX))) (Variables|FreeAim|GetMinRotX) (Variables|FreeAim|GetMaxRotX)) (.Pitch (Math|Rotator|BreakRotator (Variables|FreeAim|GetRotX))) (.Yaw (Math|Rotator|BreakRotator (Variables|FreeAim|GetRotX)))))))
      (:then_2
        (if (Variables|FreeAim|GetEnableDeadzoneY)
          (Variables|FreeAim|SetRotY (Math|Rotator|MakeRotator (+ (* (Variables|InputValues|GetVertical%20Mouse) (Variables|FreeAim|GetStartSensitivity)) (.Roll (Math|Rotator|BreakRotator (* (Variables|FreeAim|GetRotY) -1.0)))) (+ (* (Variables|InputValues|GetVertical%20Mouse) (Variables|FreeAim|GetStartSensitivity)) (.Pitch (Math|Rotator|BreakRotator (* (Variables|FreeAim|GetRotY) -1.0)))) (+ (* (Variables|InputValues|GetVertical%20Mouse) (Variables|FreeAim|GetStartSensitivity)) (.Yaw (Math|Rotator|BreakRotator (* (Variables|FreeAim|GetRotY) -1.0))))))
          (Variables|FreeAim|SetRotY (Math|Rotator|MakeRotator (.Roll (Math|Rotator|BreakRotator (* (Variables|FreeAim|GetRotY) -1.0))) (.Pitch (Math|Rotator|BreakRotator (* (Variables|FreeAim|GetRotY) -1.0))) (Math|Float|ClampAngle (.Yaw (Math|Rotator|BreakRotator (* (Variables|FreeAim|GetRotY) -1.0))) (Variables|FreeAim|GetMinRotY) (Variables|FreeAim|GetMaxRotY))))))
      (:then_3
        (Variables|FreeAim|SetDeadZoneTargetRot (Math|Rotator|MakeRotator (.yaw (Variables|FreeAim|GetRotY)) 0.0 (.roll (Variables|FreeAim|GetRotX))))
        (Transformation|SetRelativeRotation (Variables|InputValues|GetEffector%20Component) (Math|Rotator|Lerp(Rotator) (Variables|/Script/Engine.SceneComponent|GetRelativeRotation (Variables|InputValues|GetEffector%20Component)) (Variables|FreeAim|GetDeadZoneTargetRot) (* (Utilities|Time|GetWorldDeltaSeconds) (Variables|FreeAim|GetSmoothRotation)) true) false false)
        (Variables|FreeAim|SetFinalDeadzoneAimRotation (Variables|/Script/Engine.SceneComponent|GetRelativeRotation (Variables|InputValues|GetEffector%20Component))))
      (:then_4
        (if (Variables|FreeAim|GetEnableTilt)
          (Variables|FreeAim|SetTiltAroundZ (Math|Rotator|MakeRotator 0.0 0.0 (* (Variables|InputValues|GetVertical%20Mouse) (Variables|FreeAim|GetTiltingAngle))))
          (Variables|FreeAim|SetTiltAroundX (Math|Rotator|MakeRotator 0.0 (* (Variables|InputValues|GetHorizontal%20Mouse) (Variables|FreeAim|GetTiltingAngle)) 0.0))
          (Variables|FreeAim|SetTiltTargetRot (Math|Rotator|MakeRotator (.roll (Variables|FreeAim|GetTiltAroundX)) 0.0 (.yaw (Variables|FreeAim|GetTiltAroundX))))
          (Transformation|SetRelativeRotation (Variables|InputValues|GetEffector%20Component) (Math|Rotator|Lerp(Rotator) (Variables|/Script/Engine.SceneComponent|GetRelativeRotation (Variables|InputValues|GetEffector%20Component)) (Variables|FreeAim|GetTiltTargetRot) (* (Utilities|Time|GetWorldDeltaSeconds) (Variables|FreeAim|GetSmoothRotation)) true) false false))))))